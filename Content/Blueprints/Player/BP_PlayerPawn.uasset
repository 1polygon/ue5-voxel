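; Player pawn that acts as a free-fly camera and brush tool for sculpting or painting the voxel chunk from BP_World.
; BeginPlay creates the brush and VoxelEditor UI; holding right mouse switches to look-and-move, while the wheel dollies along the view.
; Otherwise, Tick places the brush under the cursor with a debug sphere.
; Left mouse applies it at a throttled rate and updates the chunk, with Shift inverting strength.
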(event `self.ReceiveBeginPlay`
  (bind _returnvalue (`GameplayStatics.GetPlayerController` 0))
  (bind _returnvalue_2 (`GameplayStatics.GetActorOfClass` "/Game/Blueprints/BP_World.BP_World_C"))
  (set `self.VoxelChunk` (`/Game/Blueprints/BP_World.VoxelChunk` _returnvalue_2))
  (`self.K2_SetActorLocation` (+ (`self.K2_GetActorLocation`) (800.0 800.0 800.0)))
  (set `PlayerController.bShowMouseCursor` true (`GameplayStatics.GetPlayerController` 0))
  (bind _returnvalue_3 (`|GenericCreateObject` "/Script/Voxel.VoxelBrush" self))
  (set `self.VoxelBrush` _returnvalue_3)
  ;[1 1 1] Add UI
  (bind _returnvalue_4 (`|CreateWidget` "/Game/UI/VoxelEditor.VoxelEditor_C" _returnvalue))
  (`UserWidget.AddToViewport` _returnvalue_4 0)
  (`WidgetBlueprintLibrary.SetInputMode_GameAndUIEx` _returnvalue null "DoNotLock" false))

(event `self.ReceiveTick`
  (params (DeltaSeconds :type "Float (single-precision)"))
  (bind _hitresult (`PlayerController.GetHitResultUnderCursorByChannel` (`GameplayStatics.GetPlayerController` 0) "TraceTypeQuery1" true))
  (if (`self.Look`)
    ;[1 1 1] Look
    (`SceneComponent.K2_AddRelativeRotation` (`self.Camera`) (`KismetMathLibrary.MakeRotator` 0.0 (`self.GetInputAxisValue`) (`self.GetInputAxisValue`)) false false)
    (`self.K2_AddActorWorldOffset` (* (`KismetMathLibrary.Normal` (+ (* (`self.GetInputAxisValue`) (`SceneComponent.GetForwardVector` (`self.Camera`))) (* (`SceneComponent.GetRightVector` (`self.Camera`)) (`self.GetInputAxisValue`)) (`KismetMathLibrary.MakeVector` 0.0 0.0 (`self.GetInputAxisValue`)))) (`self.Speed`)))
    (else
      ;[1 1 1] Sculpt/Paint
      (bind _assphere_shape (cast `SphereShape` (`VoxelBrush.Shape` (`self.VoxelBrush`))))
      (`KismetSystemLibrary.DrawDebugSphere` (`.Location` (`GameplayStatics.BreakHitResult` _hitresult)) (* (`SphereShape.Radius` _assphere_shape) 100.0))
      (set `VoxelBrush.Location` (/ (`.Location` (`GameplayStatics.BreakHitResult` _hitresult)) 100.0) (`self.VoxelBrush`))
      (if (> (- (`KismetSystemLibrary.GetGameTimeInSeconds`) (`self.LastEdit`)) (/ 1.0 (`self.EditsPerSecond`)))
        (set `self.LastEdit` (`KismetSystemLibrary.GetGameTimeInSeconds`))
        (if (`self.IsEditing`)
          (`self.ApplyBrush`))))))

(event `Key|RightMouseButton`
  (params (Key :type "Key Structure"))
  (bind _returnvalue (`GameplayStatics.GetPlayerController` 0))
  ;[1 1 1] Look
  (:`Pressed`
    (set `self.Look` true)
    (set `PlayerController.bShowMouseCursor` false _returnvalue))
  (:`Released`
    (set `self.Look` false)
    (set `PlayerController.bShowMouseCursor` true _returnvalue)))

(event `InputAxisKey|MouseWheelAxis`
  (params (AxisValue :type "Float (single-precision)"))
  ;[1 1 1] Look
  (`self.K2_AddActorWorldOffset` (* (`SceneComponent.GetForwardVector` (`self.Camera`)) (`self.Speed`) AxisValue)))

(event `Key|LeftMouseButton`
  (params (Key :type "Key Structure"))
  ;[1 1 1] Sculpt/Paint
  (:`Pressed`
    (set `self.IsEditing` true)
    (set `self.LastEdit` (`KismetSystemLibrary.GetGameTimeInSeconds`))
    (`self.ApplyBrush`))
  (:`Released`
    (set `self.IsEditing` false)))

(event `Key|LeftShift`
  (params (Key :type "Key Structure"))
  ;[1 1 1] Sculpt/Paint
  (:`Pressed`
    (set `VoxelBrush.Strength` -1.0 (`self.VoxelBrush`)))
  (:`Released`
    (set `VoxelBrush.Strength` 1.0 (`self.VoxelBrush`))))

(fn `ApplyBrush`
  (switch `/Game/UI/VoxelBrushMode` (`self.VoxelBrushMode`)
    (:`NewEnumerator0`
      (`VoxelChunk.Sculpt` (`self.VoxelChunk`) (`self.VoxelBrush`)))
    (:`NewEnumerator1`
      (`VoxelChunk.Paint` (`self.VoxelChunk`) (`self.VoxelBrush`) (`self.VoxelBrushMaterial`))))
  (`VoxelChunk.Update` (`self.VoxelChunk`)))

(fn `UserConstructionScript`)